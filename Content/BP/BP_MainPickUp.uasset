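; BP_MainPickUp is an interactable item pickup actor that moves its item into the interacting character's inventory.
; On Interact it tries to equip the item, falls back to adding it to a found inventory slot, and destroys itself if either path is taken.
; Helper functions switch the pickup text between an E-key prompt and the table row name.
; The FarInteraction overlap events are empty, leaving their cursor and look-timer logic disconnected.
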(event OnComponentBeginOverlap(FarInteraction)
  (params (OverlappedComponent :type Primitive%20Component%20Object%20Reference) (OtherActor :type Actor%20Object%20Reference) (OtherComp :type Primitive%20Component%20Object%20Reference) (OtherBodyIndex :type Integer) (bFromSweep :type Boolean) (SweepResult :type Hit%20Result%20Structure%20%28by%20ref%29)))

(event OnComponentEndOverlap(FarInteraction)
  (params (OverlappedComponent :type Primitive%20Component%20Object%20Reference) (OtherActor :type Actor%20Object%20Reference) (OtherComp :type Primitive%20Component%20Object%20Reference) (OtherBodyIndex :type Integer)))

(event EventInteract
  (params (Char :type Fight%20for%20Fame%20Character%20Object%20Reference))
  (bind _inventorymanager (Variables|/Script/FightForFame.FightForFameCharacter|GetInventoryManager Char))
  (bind _item (Variables|Default|GetItem))
  (bind _returnvalue (Class|ACInventoryManager|FindSlot _inventorymanager _item))
  (bind _returnvalue_2 (Class|ACInventoryManager|EquipItem _inventorymanager (.EquipmentSlot (Utilities|Struct|BreakItem _item)) _item -1))
  (if _returnvalue_2
    (Actor|DestroyActor :!label _label)
    (elif (not (< _returnvalue 0))
      (Class|ACInventoryManager|AddItem _inventorymanager _returnvalue _item)
      (goto _label))))

(fn ConstructionScript)

(fn SetInteractionText
  (params (NewParam :type String))
  (Rendering|Components|TextRender|SetText (Variables|Default|GetPickupText) (Utilities|Text|ToText(String) (Utilities|String|Append "Press E to pickup " NewParam))))

(fn ResetInteractionText
  (Rendering|Components|TextRender|SetText (Variables|Default|GetPickupText) (Utilities|Text|ToText(Name) (.RowName (Utilities|Struct|BreakDataTableRowHandle (Variables|Default|GetTableRow))))))